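; BPC_CharHealth is a component that tracks a character's current and maximum health.
; One tick after BeginPlay it broadcasts the starting values through the InitHealthEvent dispatcher and prints a debug string.
; TakeDamage subtracts damage, clamps health between zero and the maximum, then broadcasts both values through DamageTaken.
; The component itself has no death handling and an empty Tick.
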(event `self.ReceiveBeginPlay`
  (`KismetSystemLibrary.DelayUntilNextTick`)
  (`self.initHealth`))

(event `self.ReceiveTick`
  (params (DeltaSeconds :type "Float (single-precision)")))

(fn `initHealth`
  (`self.initHealthEvent` (`self.CurrentHealth`) (`self.MaxHealth`))
  (`KismetSystemLibrary.PrintString` "AAAAAAAAAAAA" true true (struct :`R` 1.0 :`B` 0.981161 :`A` 1.0) 5.0))

(fn `takeDamage`
  (params (Damage :type "Float (double-precision)"))
  (set `self.CurrentHealth` (`KismetMathLibrary.FClamp` (- (`self.CurrentHealth`) Damage) 0.0 (`self.MaxHealth`)))
  (`self.damageTaken` (`self.CurrentHealth`) (`self.MaxHealth`)))