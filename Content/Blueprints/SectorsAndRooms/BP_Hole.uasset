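; BP_Hole is a hole trap actor that sends a Fall call when an actor implementing BPI_Hole overlaps its trigger box.
; Its construction script applies the per-instance tilemap asset to the PaperTileMap and rotates it 90 degrees.
; It then looks up that tilemap's name in DT_HoleData to set the box's extent and position, so one Blueprint serves differently shaped holes.
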(event `self.Box.OnComponentBeginOverlap`
  (params (OverlappedComponent :type "PrimitiveComponent Object Reference") (OtherActor :type "Actor Object Reference") (OtherComp :type "PrimitiveComponent Object Reference") (OtherBodyIndex :type Integer) (bFromSweep :type Boolean) (SweepResult :type "HitResult Structure (by ref)"))
  (if (`KismetSystemLibrary.DoesImplementInterface` OtherActor "/Game/Blueprints/BPInterfaces/BPI_Hole.BPI_Hole_C")
    (`self.Fall`)
    (`KismetSystemLibrary.PrintText` "FALL SENT!" true true (struct :`R` 1.0 :`B` 0.169592 :`A` 1.0))))

(fn `UserConstructionScript`
  (bind _tile_map_asset (`self.Tile Map Asset`))
  (bind _box (`self.Box`))
  ;[1 1 1 1 36] SET TILE MAP - Permite establecer distintos tilemaps para un actor instanciado
  (`PaperTileMapComponent.SetTileMap` (`self.PaperTileMap`) _tile_map_asset)
  (`SceneComponent.K2_SetRelativeRotation` (`self.PaperTileMap`) (struct :`Roll` 90.0) false false)
  ;[1 1 1] SET BOX EXTENT & LOCATION - Determina el tamaño de la box y su ubicación en el tilemap.
  (bind _returnvalue (`|GetDataTableRow` "/Game/Blueprints/Structure/DT_HoleData.DT_HoleData" (`KismetStringLibrary.Conv_StringToName` (`KismetSystemLibrary.GetDisplayName` _tile_map_asset)))
    (:`then`
      (bind (_boxextent _boxposition) (break `/Game/Blueprints/Structure/F_HoleData` _returnvalue))
      (`BoxComponent.SetBoxExtent` _box _boxextent true)
      (`SceneComponent.K2_SetRelativeLocation` _box _boxposition false false))))