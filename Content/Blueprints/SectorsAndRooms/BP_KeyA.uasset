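; BP_KeyA is an interactable key pickup linked to a door.
; When KeyAvaible is false it hides itself on BeginPlay, disabling collision, physics and gravity until DropKey reveals it and re-enables them with a debug print.
; The construction script applies the visible physical state when KeyAvaible is true.
; Interacting sends PickUpKeyMessage to DoorToOpen, then destroys the key.
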(event `self.ReceiveBeginPlay`
  (bind _box (`self.Box`))
  (if (not (`self.bKeyAvaible?`))
    (`self.SetActorHiddenInGame` true)
    (`self.SetActorEnableCollision` false)
    (`PrimitiveComponent.SetSimulatePhysics` _box false)
    (`PrimitiveComponent.SetSimulatePhysics` (`self.Sprite`) false)
    (`PrimitiveComponent.SetEnableGravity` _box false)
    (`PrimitiveComponent.SetEnableGravity` (`self.Sprite`) false)))

(event `/Game/Blueprints/BPInterfaces/BPI_Interact.Interact!`
  (params (InteractingActor :type "/Game/Blueprints/Playable_Characters/BP_Capi Object Reference"))
  ;[1 1 1 1 36] PICK UP KEY - Toma la llave, emite una señal y destruye el actor de la llave.
  (message `/Game/Blueprints/BPInterfaces/BPI_Door.PickUpKey` (`self.DoorToOpen`))
  (`self.K2_DestroyActor`))

(event `/Game/Blueprints/BPInterfaces/BPI_Key.DropKey`
  (bind _box (`self.Box`))
  (`KismetSystemLibrary.PrintText` "DROP KEY" true true (struct :`G` 1.0 :`B` 0.029325 :`A` 1.0) 1.0)
  (`self.SetActorHiddenInGame` false)
  (`self.SetActorEnableCollision` true)
  (`PrimitiveComponent.SetSimulatePhysics` _box true)
  (`PrimitiveComponent.SetSimulatePhysics` (`self.Sprite`) true)
  (`PrimitiveComponent.SetEnableGravity` _box true)
  (`PrimitiveComponent.SetEnableGravity` (`self.Sprite`) true))

(fn `UserConstructionScript`
  (bind _box (`self.Box`))
  (if (`self.bKeyAvaible?`)
    (`self.SetActorHiddenInGame` false)
    (`self.SetActorEnableCollision` true)
    (`PrimitiveComponent.SetSimulatePhysics` _box true)
    (`PrimitiveComponent.SetSimulatePhysics` (`self.Sprite`) true)
    (`PrimitiveComponent.SetEnableGravity` _box true)
    (`PrimitiveComponent.SetEnableGravity` (`self.Sprite`) true)))