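; Camera manager that frames the current sector or room with an orthographic camera and follows the player (Capi) where the sector allows it.
; ChangeCamera stores the sector's follow settings, jumps to its map-relative center and eases ortho width to the new zoom via a timeline.
; While Capi is alive, Tick follows the player on the enabled axes.
; Y-only follow locks X to center and clamps Y between offset door positions.
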(event `self.ReceiveTick`
  (params (DeltaSeconds :type "Float (single-precision)"))
  (bind (_vdoorup_pos_x _vdoorup_pos_y) (`KismetMathLibrary.BreakVector` (`self.VDoorUP_POS`)))
  (bind (_vdoordown_pos_x _vdoordown_pos_y) (`KismetMathLibrary.BreakVector` (`self.VDoorDOWN_POS`)))
  (bind (_returnvalue_x _returnvalue_y) (`KismetMathLibrary.BreakVector` (`self.K2_GetActorLocation` (`GameplayStatics.GetPlayerCharacter` 0))))
  (bind (_returnvalue_x_2 _returnvalue_y_2) (`KismetMathLibrary.BreakVector` (`self.K2_GetActorLocation` (`GameplayStatics.GetPlayerCharacter` 0))))
  (bind _returnvalue_x_3 (`KismetMathLibrary.BreakVector` (`self.K2_GetActorLocation` (`GameplayStatics.GetPlayerCharacter` 0))))
  ;[1 1 1 1 36] CAMERA FOLLOW Y - La camara sigue el movimiento del personaje en el eje Y/X cuando un sector lo requiere.
  (if (`self.bIsCapiAlive?`)
    (`|ExecutionSequence`
      (:`then_0`
        (if (and (`self.followY?`) (`self.followX?`))
          (`self.K2_SetActorLocation` (`KismetMathLibrary.MakeVector` _returnvalue_x_2 _returnvalue_y_2))))
      (:`then_1`
        (if (and (`self.followY?`) (not (`self.followX?`)))
          (`self.K2_SetActorLocation` (`KismetMathLibrary.MakeVector` (`self.map_Center_X`) (`KismetMathLibrary.FClamp` _returnvalue_y (+ _vdoorup_pos_y (`self.Cam YUp Limit`)) (+ _vdoordown_pos_y (`self.Cam YDown Limit`)))))))
      (:`then_2`
        (if (and (`self.followX?`) (not (`self.followY?`)))
          (`self.K2_SetActorLocation` (`KismetMathLibrary.MakeVector` _returnvalue_x_3 (`self.map_Center_Y`))))))))

(event `/Game/Blueprints/BPInterfaces/BPI_Player.CapiDead!`
  (params (`bIsCapiAlive?` :type Boolean))
  ;[1 1 1 1 36] CAPI DEAD - Recibe la señal de  si Capi está vivo.
  (set `self.bIsCapiAlive?` `bIsCapiAlive?`))

(event `/Game/Blueprints/BPInterfaces/BPI_Sector.ChangeCamera`
  (params (`Camera Zoom` :type "Float (double-precision)") (`Map Camera X` :type "Float (double-precision)") (`Map Camera Y` :type "Float (double-precision)") (`Map Location` :type "Vector Structure") (`FollowX?` :type Boolean) (`FollowY?` :type Boolean) (VDoorUp_POS :type "Vector Structure") (VDoorDown_POS :type "Vector Structure") (Cam_YUp_Limit :type "Float (double-precision)") (Cam_YDown_Limit :type "Float (double-precision)"))
  (bind _returnvalue (+ `Map Camera X` `Map Location_X`))
  (bind _returnvalue_2 (+ `Map Camera Y` `Map Location_Y`))
  ;[1 1 1 1 36] CAMERA CHANGE SECTOR - Cuando el personaje ingresa a una nueva sala, mueve la cámara a la misma.
  (set `self.VDoorUP_POS` VDoorUp_POS)
  (set `self.VDoorDOWN_POS` VDoorDown_POS)
  (set `self.followX?` `FollowX?`)
  (set `self.followY?` `FollowY?`)
  (set `self.Cam YUp Limit` Cam_YUp_Limit)
  (set `self.Cam YDown Limit` Cam_YDown_Limit)
  (set `self.map_Center_X` _returnvalue)
  (set `self.map_Center_Y` _returnvalue_2)
  (`self.K2_SetActorLocation` (`KismetMathLibrary.MakeVector` _returnvalue _returnvalue_2 1000.0))
  (set `self.Camera_Width` (`CameraComponent.OrthoWidth` (`self.Camera`)))
  (set `self.new Camera Width` `Camera Zoom`)
  (`TimelineComponent.PlayFromStart` (`self.ZoomTimeline`))
  (bind (_direction _alpha) (`Timeline|ZoomTimeline` :`NewTime` 1.0)
    (:`Update`
      (set `CameraComponent.OrthoWidth` (`KismetMathLibrary.Lerp` (`self.Camera_Width`) (`self.new Camera Width`) _alpha) (`self.Camera`)))))

(fn `UserConstructionScript`)