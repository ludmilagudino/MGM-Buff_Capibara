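; Door actor that sends an interacting actor the location of its TargetDoor, or signals BP_LevelManager to end the level when it is an untargeted EndLevel door.
; Interaction requires HasKey, set by PickUpKey; Tick shows a padlock sprite while locked.
; Construction and BeginPlay snap the door to the OwnerSector component named after the sector and PlacementTag.
; Construction also sets the directional flipbook.
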(event `self.ReceiveTick`
  (params (DeltaSeconds :type "Float (single-precision)"))
  ;[1 1 1] CANDADO - Coloca o elimina el sprite de candado de cada puerta dependiendo de si la misma tiene una llave asignada.
  (if (`self.bHasKey?`)
    (`PaperSpriteComponent.SetSprite` (`self.PaperSprite`) null)
    (else
      (`PaperSpriteComponent.SetSprite` (`self.PaperSprite`) "/Game/Assets/2D/Items/Candado_Sprite.Candado_Sprite"))))

(event `self.ReceiveBeginPlay`
  ;[1 1 1 1 36] UBICAR PUERTAS - Beginplay
  (if (and (`KismetSystemLibrary.IsValid` (`self.OwnerSector`)) (!= (`self.PlacementTag`) "None"))
    (for _array_element (`self.K2_GetComponentsByClass` (`self.OwnerSector`) "/Script/Engine.SceneComponent")
      (if (== (`KismetSystemLibrary.GetDisplayName` _array_element) (`KismetStringLibrary.Conv_NameToString` (`KismetStringLibrary.Conv_StringToName` (`KismetStringLibrary.Concat_StrStr` (`KismetSystemLibrary.GetDisplayName` (`self.OwnerSector`)) "." (`KismetStringLibrary.Conv_NameToString` (`self.PlacementTag`))))))
        (`self.K2_SetActorLocation` (`SceneComponent.K2_GetComponentLocation` _array_element) false true)))))

(event `/Game/Blueprints/BPInterfaces/BPI_Door.PickUpKey`
  ;[1 1 1 1 36] ABLE DOOR - Al agarrar una llave habilita una puerta determinada
  (set `self.bHasKey?` true))

(event `/Game/Blueprints/BPInterfaces/BPI_Interact.Interact!`
  (params (InteractingActor :type "/Game/Blueprints/Playable_Characters/BP_Capi Object Reference"))
  (bind _targetdoor (`self.TargetDoor`))
  ;[1 1 1 1 36] INTERACT DOOR - Cuando un actor interactua con la puerta, se revisa si la misma puede ser utilizada y se envía su información con una señal.
  (if (`self.bHasKey?`)
    (if (`KismetSystemLibrary.IsValid` (`self.TargetDoor`))
      (message `/Game/Blueprints/BPInterfaces/BPI_Door.Door Overlaping` InteractingActor (`self.K2_GetActorLocation` _targetdoor) (`SceneComponent.K2_GetComponentLocation` (`/Game/Blueprints/SectorsAndRooms/BP_Door.Box` _targetdoor)))
      (elif (`self.bEndLevel?`)
        (bind _outactors (`GameplayStatics.GetAllActorsOfClass` "/Game/Blueprints/SectorsAndRooms/BP_LevelManager.BP_LevelManager_C"))
        (message `/Game/Blueprints/BPInterfaces/BPI_Level.EndLevel` _outactors)))))

(fn `Teleported!`
  (returns (CanTeleport :type Boolean))
  (return false))

(fn `UserConstructionScript`
  (`|ExecutionSequence`
    (:`then_0`
      ;[1 1 1] SET DOOR FLIPBOOK
      (`PaperFlipbookComponent.SetFlipbook` (`self.Sprite`) (`self.Door_Direction`)))
    (:`then_1`
      ;[1 1 1] UBICAR PUERTAS - Construction Script
      (if (and (`KismetSystemLibrary.IsValid` (`self.OwnerSector`)) (!= (`self.PlacementTag`) "None"))
        (for _array_element (`self.K2_GetComponentsByClass` (`self.OwnerSector`) "/Script/Engine.SceneComponent")
          (if (== (`KismetSystemLibrary.GetDisplayName` _array_element) (`KismetStringLibrary.Conv_NameToString` (`KismetStringLibrary.Conv_StringToName` (`KismetStringLibrary.Concat_StrStr` (`KismetSystemLibrary.GetDisplayName` (`self.OwnerSector`)) "." (`KismetStringLibrary.Conv_NameToString` (`self.PlacementTag`))))))
            (`self.K2_SetActorLocation` (`SceneComponent.K2_GetComponentLocation` _array_element))))))
    (:`then_2`
      ;[1 1 1] CANDADO - Coloca un sprite de candado a las puertas que no tienen una llave asignada.
      (if (not (`self.bHasKey?`))
        (`PaperSpriteComponent.SetSprite` (`self.PaperSprite`) "/Game/Assets/2D/Items/Candado_Sprite.Candado_Sprite")))))