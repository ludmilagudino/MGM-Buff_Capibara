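; A placeable hole actor that sends a fall message to actors overlapping it.
; On construction it applies the instance's chosen Paper2D sprite and uses that sprite's name to look up the box extent and position in DT_HoleData.
; Every tick it finds overlapping actors implementing BPI_Hole and calls FallMessage on them when a component overlapping the box has a display name matching PjCollisionElement.
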(event `self.ReceiveTick`
  (params (DeltaSeconds :type "Float (single-precision)"))
  ;[1 1 1] FALL - Detecta si hay algun actor colisionando contra la box y si el mismo implementa la BPI_Hole. Posteriormente, si el nombre de alguno de los componentes que hacen overlap coincide con el valor de la variable pjCollisionElement, envía la señal FALL.
  (for _array_element (`self.GetOverlappingActors` "/Script/Engine.Actor")
    (if (`KismetSystemLibrary.DoesImplementInterface` _array_element "/Game/Blueprints/BPInterfaces/BPI_Hole.BPI_Hole_C")
      (for _array_element_2 (`PrimitiveComponent.GetOverlappingComponents` (`self.Box`))
        (if (== (`KismetSystemLibrary.GetDisplayName` _array_element_2) (`self.pjCollisionElement`))
          (message `/Game/Blueprints/BPInterfaces/BPI_Hole.Fall` _array_element)
          (`KismetSystemLibrary.PrintText` "FALL SENT!" true true (struct :`R` 1.0 :`B` 0.169592 :`A` 1.0)))))))

(fn `UserConstructionScript`
  (bind _paper_spritea (`self.paper SpriteA`))
  (bind _box (`self.Box`))
  ;[1 1 1 1 36] SET PAPER SPRITE - Permite establecer distintos sprites para un actor instanciado
  (`PaperSpriteComponent.SetSprite` (`self.PaperSprite`) _paper_spritea)
  ;[1 1 1] SET BOX EXTENT & LOCATION - Determina el tamaño de la box y su ubicación en el sprite.
  (bind _returnvalue (`|GetDataTableRow` "/Game/Blueprints/Structure/DT_HoleData.DT_HoleData" (`KismetStringLibrary.Conv_StringToName` (`KismetSystemLibrary.GetDisplayName` _paper_spritea)))
    (:`then`
      (bind (_boxextent _boxposition) (break `/Game/Blueprints/Structure/F_HoleData` _returnvalue))
      (`BoxComponent.SetBoxExtent` _box _boxextent true)
      (`SceneComponent.K2_SetRelativeLocation` _box _boxposition false false))))