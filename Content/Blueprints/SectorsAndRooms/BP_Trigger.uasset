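; BP_Trigger is a box trigger that starts Vizcacha mother or tutorial messages when the player enters it.
; On overlap by an actor implementing BPI_Player, it finds BP_LevelManager and calls the message functions enabled by its two boolean flags.
; Each flag clears so its message fires once, with a short delay before the Vizcacha one.
; End overlap does nothing, as the hide-and-rearm tutorial logic is disconnected.
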(event `self.Box.OnComponentBeginOverlap`
  (params (OverlappedComponent :type "PrimitiveComponent Object Reference") (OtherActor :type "Actor Object Reference") (OtherComp :type "PrimitiveComponent Object Reference") (OtherBodyIndex :type Integer) (bFromSweep :type Boolean) (SweepResult :type "HitResult Structure (by ref)"))
  (if (`KismetSystemLibrary.DoesImplementInterface` OtherActor "/Game/Blueprints/BPInterfaces/BPI_Player.BPI_Player_C")
    (bind _outactors (`GameplayStatics.GetAllActorsOfClass` "/Game/Blueprints/SectorsAndRooms/BP_LevelManager.BP_LevelManager_C"))
    (`|ExecutionSequence`
      (:`then_0`
        (if (`self.bVizcachaConvo?`)
          (set `self.bVizcachaConvo?` false)
          (`KismetSystemLibrary.Delay` 0.4)
          (message `/Game/Blueprints/BPInterfaces/BPI_Dialogue.VizcachaMadre` _outactors)))
      (:`then_1`
        (if (`self.bTutorialConvo?`)
          (message `/Game/Blueprints/BPInterfaces/BPI_Dialogue.ShowTutorial` _outactors)
          (set `self.bTutorialConvo?` false))))))

(event `self.Box.OnComponentEndOverlap`
  (params (OverlappedComponent :type "PrimitiveComponent Object Reference") (OtherActor :type "Actor Object Reference") (OtherComp :type "PrimitiveComponent Object Reference") (OtherBodyIndex :type Integer)))

(fn `UserConstructionScript`)