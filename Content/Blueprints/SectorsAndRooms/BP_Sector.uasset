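; BP_Sector is a tilemap room that manages camera settings, enemy activation and a key drop.
; Construction reads the tilemap's DT_SectorData row to size the trigger, set camera values, center the box and position four door points.
; Overlapping characters receive room and camera data, while enemies gathered after BeginPlay activate on entry and deactivate on exit.
; EnemyDied shrinks that array by index, not identity, and once empty Tick signals BPKey to drop once.
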(event `self.ReceiveTick`
  (params (DeltaSeconds :type "Float (single-precision)"))
  ;[1 1 1 1 36] DROP KEY - Envia una señal para que el BP_Key active sus físicas y caiga adentro del sector.
  (if (`self.bAllEnemiesDead`)
    (if (not (`self.bKeyDropped?`))
      (message `/Game/Blueprints/BPInterfaces/BPI_Key.DropKey` (`self.BP_Key`))
      (set `self.bKeyDropped?` true))))

(event `self.ReceiveBeginPlay`
  ;[1 1 1 1 36] COUNT ENEMIES -  Cada sector genera un array con la cantidad de enemigos que están en su espacio.
  (`KismetSystemLibrary.Delay` 1.0)
  (bind _output_get (set `self.enemiesInRoom` (`PrimitiveComponent.GetOverlappingActors` (`self.Box Trigger`) "/Game/Blueprints/Enemies/BP_EnemyBaseZD.BP_EnemyBaseZD_C")))
  (for _array_element _output_get
    (`KismetSystemLibrary.PrintText` (`KismetTextLibrary.Conv_ObjectToText` _array_element) true true (struct :`R` 1.0 :`G` 0.842401 :`B` 0.285186 :`A` 1.0) 6.0))
  (set `self.bKeyDropped?` false))

(event `self.Box Trigger.OnComponentBeginOverlap`
  (params (OverlappedComponent :type "PrimitiveComponent Object Reference") (OtherActor :type "Actor Object Reference") (OtherComp :type "PrimitiveComponent Object Reference") (OtherBodyIndex :type Integer) (bFromSweep :type Boolean) (SweepResult :type "HitResult Structure (by ref)"))
  ;[1 1 1 1 36] CAPI ENTER - Detecta cuando Capi ingresa a un sector y comparte información del mismo mediante la señal Enter Room.
  (if (`KismetSystemLibrary.DoesImplementInterface` OtherActor "/Game/Blueprints/BPInterfaces/BPI_Characters.BPI_Characters_C")
    (message `/Game/Blueprints/BPInterfaces/BPI_Sector.EnterRoom` OtherActor (`self.bUsePlayerCam?`) (`self.CameraZoom`) (`KismetMathLibrary.Conv_IntToDouble` (`self.Map X Center`)) (`KismetMathLibrary.Conv_IntToDouble` (`self.Map Y Center`)) (`self.K2_GetActorLocation`) (`self.Cam Follow X`) (`self.Cam Follow Y`) (`self.VDoorUP_POS`) (`self.VDoorDOWN_POS`) (`self.Cam YUp Limit`) (`self.Cam YDown Limit`))
    ;[1 1 1 1 36] ENEMIES ACTIVATE - Activa a cada enemigo detectado en el sector.
    (for _array_element (`self.enemiesInRoom`)
      (message `/Game/Blueprints/BPInterfaces/BPI_Enemy.EnemiesActivate!` _array_element true)
      (`KismetSystemLibrary.PrintText` (`KismetTextLibrary.Conv_StringToText` (`KismetStringLibrary.Conv_ObjectToString` _array_element)) true true (struct :`R` 1.0 :`B` 0.178082 :`A` 1.0) 4.0))))

(event `self.Box Trigger.OnComponentEndOverlap`
  (params (OverlappedComponent :type "PrimitiveComponent Object Reference") (OtherActor :type "Actor Object Reference") (OtherComp :type "PrimitiveComponent Object Reference") (OtherBodyIndex :type Integer))
  ;[1 1 1 1 36] CAPI EXIT - Detecta cuando Capi sale de un sector
  (if (`KismetSystemLibrary.DoesImplementInterface` OtherActor "/Game/Blueprints/BPInterfaces/BPI_Characters.BPI_Characters_C")
    (for _array_element (`self.enemiesInRoom`)
      (if (`KismetSystemLibrary.IsValid` _array_element)
        (message `/Game/Blueprints/BPInterfaces/BPI_Enemy.EnemiesDeactivate!` _array_element false)))))

(event `/Game/Blueprints/BPInterfaces/BPI_Enemy.EnemyDied`
  (bind _enemiesinroom (`self.enemiesInRoom`))
  ;[1 1 1 1 36] ENEMIE DIE - Remueve un elemento del array de enemigos por cada uno que es vencido. Si el array llega a 0 se activa el booleano All Enemies Dead.
  (`KismetArrayLibrary.Array_Remove` _enemiesinroom)
  (if (> (`KismetArrayLibrary.Array_Length` _enemiesinroom) 0)
    (for _array_element (`self.enemiesInRoom`)
      _)
    (else
      (`KismetSystemLibrary.PrintText` "All dead!" true true (struct :`R` 0.667645 :`G` 0.82166 :`B` 1.0 :`A` 1.0) 4.0)
      (set `self.bAllEnemiesDead` true))))

(fn `UserConstructionScript`
  (bind _up (`self.UP`))
  (bind _down (`self.DOWN`))
  (bind _tilemapasset (`self.TileMapAsset`))
  (bind _tilemapasset_2 (`self.TileMapAsset`))
  ;[1 1 1 1 36] ELECCIÓN DE TILEMAP - Mediante una tabla determina que tilemap elegir. Posteriormente, revisa las medidas del box trigger y el ancho de la camara que corresponden a dicho tilemap. Algunas cosas sobran y se puede mejorar, pero funiona.
  (`PaperTileMapComponent.SetTileMap` (`self.PaperTileMap`) _tilemapasset)
  (bind _returnvalue (`|GetDataTableRow` "/Game/Blueprints/Structure/DT_SectorData.DT_SectorData" (`KismetStringLibrary.Conv_StringToName` (`KismetSystemLibrary.GetDisplayName` _tilemapasset)))
    (:`then`
      (bind (_sectortype _boxextent _camerazoom _bcamfollowx _bcamfollowy _cam_yup_limit _cam_ydown_limit) (break `/Game/Blueprints/Structure/F_SectorData` _returnvalue))
      (`BoxComponent.SetBoxExtent` (`self.Box Trigger`) _boxextent true)
      ;[1 1 1 1 36] SET VAR - Se configuran variables de DT_SectorData
      (set `self.CameraZoom` _camerazoom)
      (set `self.Cam Follow X` _bcamfollowx)
      (set `self.Cam Follow Y` _bcamfollowy)
      (set `self.Cam YUp Limit` _cam_yup_limit)
      (set `self.Cam YDown Limit` _cam_ydown_limit)
      ;[1 1 1 1 36] CENTRAR COLLISION BOX - Toma el tamaño del tilemap en tiles y las medidas de un tile. Posteriormente, calcula donde está el centro del tilemap para ubicar el box trigger. Este trigger actualmente se utiliza para controlar el zoom de la cámara.
      (bind (_mapwidth _mapheight) (`PaperTileMapComponent.GetMapSize` (`self.PaperTileMap`)))
      (bind _output_get (set `self.Map Width` _mapwidth))
      (bind _output_get_2 (set `self.Map Height` _mapheight))
      (bind _output_get_3 (set `self.Map Y Center` (- (/ (* _output_get_2 (`PaperTileMap.TileHeight` _tilemapasset_2)) 2) 64)))
      (bind _output_get_4 (set `self.Map X Center` (- (/ (* _output_get (`PaperTileMap.TileWidth` _tilemapasset_2)) 2) 64)))
      (`SceneComponent.K2_SetRelativeLocation` (`self.Box Trigger`) (`KismetMathLibrary.MakeVector` (`KismetMathLibrary.Conv_IntToDouble` _output_get_4) (`KismetMathLibrary.Conv_IntToDouble` _output_get_3) 5.0) false false)
      ;[1 1 1 1 36] ALINEAR POSICIÓN PUERTAS - Determina 4 puntos específicos de la sala en los cuales pueden instanciarse puertas. Los puntos de cada sala pueden se modificados desde el editor.
      (bind _output_get_5 (set `self.VDoorUP` (`KismetMathLibrary.MakeVector` (+ (`KismetMathLibrary.Conv_IntToDouble` (* (`self.Map Width`) 64)) -64.0) 384.0 10.0)))
      (`SceneComponent.K2_SetRelativeLocation` _up _output_get_5 false false)
      (set `self.VDoorUP_POS` (`SceneComponent.K2_GetComponentLocation` _up))
      (bind _output_get_6 (set `self.VDoorRight` (`KismetMathLibrary.MakeVector` (`KismetMathLibrary.Conv_IntToDouble` (- (* (`self.Map Width`) 128) 512)) (`KismetMathLibrary.Conv_IntToDouble` (- (* (`self.Map Height`) 64) 64)) 10.0)))
      (`SceneComponent.K2_SetRelativeLocation` (`self.RIGHT`) _output_get_6 false false)
      (bind _output_get_7 (set `self.VDoorDown` (`KismetMathLibrary.MakeVector` (`KismetMathLibrary.Conv_IntToDouble` (- (* (`self.Map Width`) 64) 64)) (`KismetMathLibrary.Conv_IntToDouble` (- (* (`self.Map Height`) 128) 512)) 10.0)))
      (`SceneComponent.K2_SetRelativeLocation` _down _output_get_7 false false)
      (set `self.VDoorDOWN_POS` (`SceneComponent.K2_GetComponentLocation` _down))
      (bind _output_get_8 (set `self.VDoorLeft` (`KismetMathLibrary.MakeVector` 384.0 (`KismetMathLibrary.Conv_IntToDouble` (- (* (`self.Map Height`) 64) 64)) 10.0)))
      (`SceneComponent.K2_SetRelativeLocation` (`self.LEFT`) _output_get_8 false false))))