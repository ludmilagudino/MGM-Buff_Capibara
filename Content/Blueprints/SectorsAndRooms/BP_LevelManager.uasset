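; BP_LevelManager is a level manager that handles per-level music, the tutorial dialogue and progression to the next level.
; On BeginPlay it matches the current level name to play that level's track and set the next destination, chaining Town, LVL_1, the boss level and Menu.
; Tutorial events show or remove the WBP_DialogueCapi widget, switching input mode and mouse cursor.
; EndLevel waits briefly, runs a "gc" console command, then opens the next level.
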(event `self.ReceiveBeginPlay`
  ;[1 1 1] SETEAR VARIABLES DE INICIO - Acá hay que colocar la música de cuando inicia cada nivel
  (bind _returnvalue (`GameplayStatics.GetCurrentLevelName` true))
  (`|ExecutionSequence`
    (:`then_0`
      (if (== _returnvalue "Town")
        (`GameplayStatics.PlaySound2D` "/Game/Assets/Sound/Demos/Demo_Pueblo_V4.Demo_Pueblo_V4" 0.3 1.0 0.0 null null)
        (set `self.NextLevelName` "LVL_1")))
    (:`then_1`
      (if (== _returnvalue "LVL_1")
        (`GameplayStatics.PlaySound2D` "/Game/Assets/Sound/Demos/Demo_Madriguera_V2.Demo_Madriguera_V2" 0.3 1.0 0.0 null null)
        (set `self.NextLevelName` "LVL_1Boss")))
    (:`then_2`
      (if (== _returnvalue "LVL_1BOSS")
        (`GameplayStatics.PlaySound2D` "/Game/Assets/Sound/OST/Buff_Capibara_Track_3_Boss_Fight.Buff_Capibara_Track_3_Boss_Fight" 0.3 1.0 0.0 null null)
        (set `self.NextLevelName` "Menu")))))

(event `/Game/Blueprints/BPInterfaces/BPI_Dialogue.ShowTutorial`
  (bind _returnvalue (`GameplayStatics.GetPlayerController` 0))
  (bind _returnvalue_2 (`|CreateWidget` "/Game/Blueprints/Widgets/WBP_DialogueCapi.WBP_DialogueCapi_C" _returnvalue))
  (bind _output_get (set `self.WPB_Dialogue` _returnvalue_2))
  (`UserWidget.AddToViewport` _output_get 0)
  (`WidgetBlueprintLibrary.SetInputMode_GameAndUIEx` _returnvalue (`self.WPB_Dialogue`))
  (set `PlayerController.bShowMouseCursor` true _returnvalue))

(event `/Game/Blueprints/BPInterfaces/BPI_Dialogue.HideTutorial`
  (bind _returnvalue (`GameplayStatics.GetPlayerController` 0))
  (`Widget.RemoveFromParent` (`self.WPB_Dialogue`))
  (`WidgetBlueprintLibrary.SetInputMode_GameOnly` _returnvalue)
  (set `PlayerController.bShowMouseCursor` false _returnvalue))

(event `/Game/Blueprints/BPInterfaces/BPI_Level.EndLevel`
  ;[1 1 1] END LEVEL - Te lleva al siguiente nivel, dependiendo del nivel en el que te encuentres.
  (`KismetSystemLibrary.Delay` 0.5)
  (`KismetSystemLibrary.ExecuteConsoleCommand` "gc" null)
  (`GameplayStatics.OpenLevel` (`self.NextLevelName`)))

(fn `UserConstructionScript`)