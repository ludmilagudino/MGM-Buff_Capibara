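; BP_Capi is the player character, with Enhanced Input movement, sprint and jump, plus a health system.
; Movement follows world X/Y axes, while stored direction and running state are available for animation; sprint switches max walk speed.
; BeginPlay adds the input mapping and creates WBP_HUD, whose health bar refreshes after Damage or Cure.
; Both clamp health, but Damage computes damage minus current health rather than the reverse.
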(event `self.ReceiveTick`
  (params (DeltaSeconds :type "Float (single-precision)")))

(event `self.ReceiveBeginPlay`
  (bind _asplayer_controller (cast `PlayerController` (`self.GetController`)))
  (`EnhancedInputSubsystemInterface.AddMappingContext` (pcsubsystem `EnhancedInputLocalPlayerSubsystem` _asplayer_controller) "/Game/Entries/InputMapping_Character.InputMapping_Character" 0 (struct))
  (`self.CreateHUD`))

(event `EnhancedInput|/Game/Entries/Inputs/IA_Move`
  (params (ActionValue :type "Vector2D Structure") (ElapsedSeconds :type "Float (double-precision)") (TriggeredSeconds :type "Float (double-precision)") (InputAction :type "InputAction Object Reference" :default "/Game/Entries/Inputs/IA_Move.IA_Move"))
  (bind (_x _y) (`KismetMathLibrary.BreakVector2D` ActionValue))
  ;[1 1 1] MOVE: Determina la velocida y dirección del movimiento del personaje. Además guarda la dirección para usar en animaciones.
  (:`Triggered`
    (set `self.Direction` ActionValue)
    (`self.AddMovementInput` (1.0 0.0 0.0) _x)
    (`self.AddMovementInput` (0.0 1.0 0.0) _y)))

(event `EnhancedInput|/Game/Entries/Inputs/IA_Run`
  (params (ActionValue :type Boolean) (ElapsedSeconds :type "Float (double-precision)") (TriggeredSeconds :type "Float (double-precision)") (InputAction :type "InputAction Object Reference" :default "/Game/Entries/Inputs/IA_Run.IA_Run"))
  (bind _charactermovement (`self.CharacterMovement`))
  ;[0.5748 0.7806 1] SPRINT: Duplica la velocidad máxima al apretar Shift izquierdo y la reduce a la mitad al soltar.
  (:`Started`
    (set `self.bIsRunning` ActionValue)
    (set `CharacterMovementComponent.MaxWalkSpeed` 1000.0 _charactermovement))
  (:`Completed`
    (set `self.bIsRunning` ActionValue)
    (set `CharacterMovementComponent.MaxWalkSpeed` 600.0 _charactermovement)))

(event `EnhancedInput|/Game/Entries/Inputs/IA_Jump`
  (params (ActionValue :type Boolean) (ElapsedSeconds :type "Float (double-precision)") (TriggeredSeconds :type "Float (double-precision)") (InputAction :type "InputAction Object Reference" :default "/Game/Entries/Inputs/IA_Jump.IA_Jump"))
  ;[1 0.9451 0.349] SALTAR: Desplazamineto vertical.
  (:`Triggered`
    (`self.Jump`)
    (set `self.JumpMaxCount` 1)))

(fn `CreateHUD`
  (locals (NewLocalVar :type "/Game/Blueprints/Widgets/WBP_HUD Object Reference"))
  (bind _returnvalue (`|CreateWidget` "/Game/Blueprints/Widgets/WBP_HUD.WBP_HUD_C" (`GameplayStatics.GetPlayerController` 0)))
  (`UserWidget.AddToViewport` _returnvalue 0)
  (bind _output_get (set `self.WBP_HUD` _returnvalue))
  (bind _wpb_healthbar (`/Game/Blueprints/Widgets/WBP_HUD.WPB_HealthBar` _output_get))
  (`ProgressBar.SetPercent` (`/Game/Blueprints/Widgets/WPB_HealthBar.ProgressBar_Health` _wpb_healthbar) (/ (`self.CurrentHealth`) (`self.MaxHealth`)))
  (set `TextBlock.Text` (`KismetTextLibrary.Conv_DoubleToText` (`self.CurrentHealth`) "HalfToEven") (`/Game/Blueprints/Widgets/WPB_HealthBar.TextCurrentHealth` _wpb_healthbar))
  (set `TextBlock.Text` (`KismetTextLibrary.Conv_DoubleToText` (`self.MaxHealth`) "HalfToEven") (`/Game/Blueprints/Widgets/WPB_HealthBar.TextMaxHealth` _wpb_healthbar)))

(fn `Cure`
  (params (Cure :type "Float (double-precision)"))
  (set `self.CurrentHealth` (`KismetMathLibrary.FClamp` (+ (`self.CurrentHealth`) Cure) 0.0 (`self.MaxHealth`)))
  (`self.UpdateWidget`))

(fn `Damage`
  (params (Damage :type "Float (double-precision)"))
  (set `self.CurrentHealth` (`KismetMathLibrary.FClamp` (- Damage (`self.CurrentHealth`)) 0.0 (`self.MaxHealth`)))
  (`self.UpdateWidget`))

(fn `UpdateWidget`
  (bind _wpb_healthbar (`/Game/Blueprints/Widgets/WBP_HUD.WPB_HealthBar` (`self.WBP_HUD`)))
  (`ProgressBar.SetPercent` (`/Game/Blueprints/Widgets/WPB_HealthBar.ProgressBar_Health` _wpb_healthbar) (/ (`self.CurrentHealth`) (`self.MaxHealth`)))
  (set `TextBlock.Text` (`KismetTextLibrary.Conv_DoubleToText` (`self.CurrentHealth`) "HalfToEven") (`/Game/Blueprints/Widgets/WPB_HealthBar.TextCurrentHealth` _wpb_healthbar))
  (set `TextBlock.Text` (`KismetTextLibrary.Conv_DoubleToText` (`self.MaxHealth`) "HalfToEven") (`/Game/Blueprints/Widgets/WPB_HealthBar.TextMaxHealth` _wpb_healthbar)))

(fn `UserConstructionScript`
  (`parent.UserConstructionScript`))