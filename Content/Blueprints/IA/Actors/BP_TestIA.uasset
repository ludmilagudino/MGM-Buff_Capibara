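; BP_TestIA is a test AI enemy Blueprint that deals melee-style hitbox damage to BP_Capi actors.
; The CheckAttack event calls EnemyAttack, which queries Hitbox0 for overlapping BP_Capi actors, applies fixed damage to each and prints its name.
; Nothing in this graph triggers CheckAttack; the default events are inactive, and an IsAttacking check and a second damage call are left unconnected.
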(event `/Game/Blueprints/BPInterfaces/BPI_Player.CheckAttack`
  (`self.Enemy Attack`))

(fn `Enemy Attack`
  (for _array_element (`PrimitiveComponent.GetOverlappingActors` (`self.Hitbox_0`) "/Game/Blueprints/Playable_Characters/BP_Capi.BP_Capi_C")
    (`GameplayStatics.ApplyDamage` _array_element 30.0)
    (`KismetSystemLibrary.PrintString` (`KismetSystemLibrary.GetDisplayName` _array_element))))

(fn `UserConstructionScript`
  (`parent.UserConstructionScript`))