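; Melee enemy Blueprint for the Escuerzo, which damages BP_Capi actors and reacts to hits and death.
; CheckAttack runs EnemyAttack, which applies fixed damage to each BP_Capi overlapping Hitbox0, prints its name and plays the melee animation.
; BPC_CharHealth events drive the hurt animation and death, where movement stops, the death animation plays and the actor is destroyed after a short delay.
; All animations play as overrides on the AnimationComponent's AnimInstance.
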(event `/Game/Blueprints/BPInterfaces/BPI_Player.CheckAttack`
  ;[1 1 1] Ataque del enemigo
  (`self.Enemy Attack`))

(event `self.BPC_CharHealth.damageTaken`
  (params (CurrentHealth :type "Float (double-precision)") (MaxHealth :type "Float (double-precision)"))
  ;[1 1 1] Recibir ataque
  (`PaperZDAnimInstance.K2_PlayAnimationOverride` (`PaperZDAnimationComponent.AnimInstance` (`self.AnimationComponent`)) "/Game/Assets/2D/Characters/PJ_EM1_Escuerzo/Animations/AnimSequences/Ani_RecieveDamage_Escuerzo.Ani_RecieveDamage_Escuerzo" "DefaultSlot" 1.0 0.0))

(event `self.BPC_CharHealth.Ondeath`
  ;[1 1 1] Muerte
  (`CharacterMovementComponent.SetMovementMode` (`self.CharacterMovement`) "MOVE_None" 0)
  (`NavMovementComponent.StopActiveMovement` (`self.CharacterMovement`))
  (`PaperZDAnimInstance.K2_PlayAnimationOverride` (`PaperZDAnimationComponent.AnimInstance` (`self.AnimationComponent`)) "/Game/Assets/2D/Characters/PJ_EM1_Escuerzo/Animations/AnimSequences/Ani_Death_Escuerzo.Ani_Death_Escuerzo" "DefaultSlot" 1.0 0.0)
  (`KismetSystemLibrary.Delay` 0.4)
  (`self.K2_DestroyActor`))

(fn `Enemy Attack`
  (for _array_element (`PrimitiveComponent.GetOverlappingActors` (`self.Hitbox_0`) "/Game/Blueprints/Playable_Characters/BP_Capi.BP_Capi_C")
    (`GameplayStatics.ApplyDamage` _array_element 30.0)
    (`KismetSystemLibrary.PrintString` (`KismetSystemLibrary.GetDisplayName` _array_element))
    (`PaperZDAnimInstance.K2_PlayAnimationOverride` (`PaperZDAnimationComponent.AnimInstance` (`self.AnimationComponent`)) "/Game/Assets/2D/Characters/PJ_EM1_Escuerzo/Animations/AnimSequences/Ani_Melee_Escuerzo.Ani_Melee_Escuerzo" "DefaultSlot" 1.0 0.0)))

(fn `UserConstructionScript`
  (`parent.UserConstructionScript`))