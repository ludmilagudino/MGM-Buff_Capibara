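; Enemy AI controller that runs the BT_Enemy behavior tree on possession and tracks the BP_Capi character through AI perception.
; Perception updates are filtered by a cast to BP_Capi, then set that actor as a blackboard object when sensed, or clear the key when lost.
; Both outcomes print a debug message, and a Spanish note proposes replacing the cast with an interface or direct character call.
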(event `self.ReceivePossess`
  (params (PossessedPawn :type "Pawn Object Reference"))
  (`self.RunBehaviorTree` "/Game/Blueprints/IA/BT_Enemy.BT_Enemy"))

(event `self.AIPerception.OnTargetPerceptionUpdated`
  (params (Actor :type "Actor Object Reference") (Stimulus :type "AIStimulus Structure"))
  (bind _asbp_capi (cast `/Game/Blueprints/Playable_Characters/BP_Capi` Actor)) ; Cambiarlo por una interfaz o llamar directamente al personaje
  (if Stimulus_bSuccessfullySensed
    (`BlackboardComponent.SetValueAsObject` (`AIBlueprintHelperLibrary.GetBlackboard` null) (`self.Key Name_1`) _asbp_capi)
    (`KismetSystemLibrary.PrintString` "Target in sight")
    (else
      (`BlackboardComponent.SetValueAsObject` (`AIBlueprintHelperLibrary.GetBlackboard` null) (`self.Key Name_1`) null)
      (`KismetSystemLibrary.PrintString` "Target lost"))))

(fn `UserConstructionScript`)