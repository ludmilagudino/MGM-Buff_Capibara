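; BP_Capi_Testing is a player character Blueprint, named as a test version, that handles basic walking, sprinting and jumping.
; BeginPlay adds the InputMapping_Character context to the Enhanced Input subsystem of its player controller.
; Walk actions move it along fixed world X and Y axes, independent of camera or actor rotation.
; Run raises max walk speed while held and tracks IsRunning, and Jump sets a single-jump limit after jumping.
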(event `self.ReceiveBeginPlay`
  (bind _asplayer_controller (cast `PlayerController` (`self.GetController`)))
  (`EnhancedInputSubsystemInterface.AddMappingContext` (pcsubsystem `EnhancedInputLocalPlayerSubsystem` _asplayer_controller) "/Game/Entries/InputMapping_Character.InputMapping_Character" 0 (struct)))

(event `EnhancedInput|/Game/Entries/Inputs/IA_WalkH`
  (params (ActionValue :type "Float (double-precision)") (ElapsedSeconds :type "Float (double-precision)") (TriggeredSeconds :type "Float (double-precision)") (InputAction :type "InputAction Object Reference" :default "/Game/Entries/Inputs/IA_WalkH.IA_WalkH"))
  ;[0.5991 1 0.8359] WALKH: Movimiento horizontal base del personaje
  (:`Triggered`
    (`self.AddMovementInput` (1.0 0.0 0.0) ActionValue)))

(event `EnhancedInput|/Game/Entries/Inputs/IA_WalkV`
  (params (ActionValue :type "Float (double-precision)") (ElapsedSeconds :type "Float (double-precision)") (TriggeredSeconds :type "Float (double-precision)") (InputAction :type "InputAction Object Reference" :default "/Game/Entries/Inputs/IA_WalkV.IA_WalkV"))
  ;[0.5991 1 0.8359] WALKV: Movimiento vertical base del personaje
  (:`Triggered`
    (`self.AddMovementInput` (0.0 1.0 0.0) ActionValue)))

(event `EnhancedInput|/Game/Entries/Inputs/IA_Run`
  (params (ActionValue :type Boolean) (ElapsedSeconds :type "Float (double-precision)") (TriggeredSeconds :type "Float (double-precision)") (InputAction :type "InputAction Object Reference" :default "/Game/Entries/Inputs/IA_Run.IA_Run"))
  (bind _charactermovement (`self.CharacterMovement`))
  ;[0.5748 0.7806 1] SPRINT: Duplica la velocidad máxima al apretar Shift izquierdo y la reduce a la mitad al soltar.
  (:`Started`
    (set `self.bIsRunning` ActionValue)
    (set `CharacterMovementComponent.MaxWalkSpeed` 1000.0 _charactermovement))
  (:`Completed`
    (set `self.bIsRunning` ActionValue)
    (set `CharacterMovementComponent.MaxWalkSpeed` 600.0 _charactermovement)))

(event `EnhancedInput|/Game/Entries/Inputs/IA_Jump`
  (params (ActionValue :type Boolean) (ElapsedSeconds :type "Float (double-precision)") (TriggeredSeconds :type "Float (double-precision)") (InputAction :type "InputAction Object Reference" :default "/Game/Entries/Inputs/IA_Jump.IA_Jump"))
  ;[1 0.9451 0.349] SALTAR: Desplazamineto vertical.
  (:`Triggered`
    (`self.Jump`)
    (set `self.JumpMaxCount` 1)))

(fn `UserConstructionScript`)