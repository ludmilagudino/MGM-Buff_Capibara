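; Ranged rat enemy Blueprint that fires projectiles at the BP_Capi player and plays attack, hit and death animation overrides.
; AttackRange only plays the attack animation; EnemyRangeNotify separately spawns the projectile ahead of the enemy at a fixed height, with velocity aimed at the player.
; BPC_CharHealth events drive hit and death reactions.
; Death stops movement, then after a short delay destroys the actor and notifies BPSector.
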(event `/Game/Blueprints/BPInterfaces/BPI_AttackRange.AttackRange`
  ;[1 1 1] Animacion de ataque
  (`self.Range Attack`))

(event `self.BPC_CharHealth.damageTaken`
  (params (CurrentHealth :type "Float (double-precision)") (MaxHealth :type "Float (double-precision)"))
  ;[1 1 1] Recibir ataque
  (`PaperZDAnimInstance.K2_PlayAnimationOverride` (`PaperZDAnimationComponent.AnimInstance` (`self.AnimationComponent`)) "/Game/Assets/2D/Characters/PJ_ER1_Rata/Animations/AnimSequences/Ani_Rata_RecieveDamage.Ani_Rata_RecieveDamage" "DefaultSlot" 1.0 0.0))

(event `self.BPC_CharHealth.Ondeath`
  ;[1 1 1] Muerte
  (`CharacterMovementComponent.SetMovementMode` (`self.CharacterMovement`) "MOVE_None" 0)
  (`NavMovementComponent.StopActiveMovement` (`self.CharacterMovement`))
  (`PaperZDAnimInstance.K2_PlayAnimationOverride` (`PaperZDAnimationComponent.AnimInstance` (`self.AnimationComponent`)) "/Game/Assets/2D/Characters/PJ_ER1_Rata/Animations/AnimSequences/Ani_Rata_Death.Ani_Rata_Death" "DefaultSlot" 1.0 0.0)
  (`KismetSystemLibrary.Delay` 0.4)
  (`self.K2_DestroyActor`)
  (message `/Game/Blueprints/BPInterfaces/BPI_Enemy.EnemyDied` (`self.BP_Sector`)))

(event `/Game/Blueprints/BPInterfaces/BPI_Notify_EnemyRange.Enemy Range Notify`
  (bind (_returnvalue_x _returnvalue_y) (`KismetMathLibrary.BreakVector` (+ (`self.K2_GetActorLocation`) (* (`self.GetActorForwardVector`) 100.0))))
  ;[1 1 1] Spawneo de projectil de enemigo
  (bind _asbp_capi (cast `/Game/Blueprints/Playable_Characters/BP_Capi` (`GameplayStatics.GetPlayerCharacter` 0)))
  (`|SpawnActorFromClass` "/Game/Blueprints/Enemies/EnemyRange/BP_Projectile_EnemyRange.BP_Projectile_EnemyRange_C" (`KismetMathLibrary.MakeTransform` (`KismetMathLibrary.MakeVector` _returnvalue_x _returnvalue_y 70.0)) "AlwaysSpawn" "MultiplyWithRoot" null (* (`KismetMathLibrary.Normal` (- (`self.K2_GetActorLocation` _asbp_capi) (`self.K2_GetActorLocation`))) (`self.ProjectileSpeed`)) null)
  (`KismetSystemLibrary.PrintString` "SPAWNEO BALA"))

(fn `Range Attack`
  (`PaperZDAnimInstance.K2_PlayAnimationOverride` (`PaperZDAnimationComponent.AnimInstance` (`self.AnimationComponent`)) "/Game/Assets/2D/Characters/PJ_ER1_Rata/Animations/AnimSequences/Ani_Rata_Range.Ani_Rata_Range" "DefaultSlot" 1.0 0.0)
  (`KismetSystemLibrary.PrintString` "ANIMACION RANGO"))

(fn `UserConstructionScript`
  (`parent.UserConstructionScript`))