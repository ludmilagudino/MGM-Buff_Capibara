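; BP_EnemyBaseZD is a base enemy Blueprint that takes damage and deals contact damage to actors it overlaps.
; AnyDamage defers to the parent class, then prints the current health from BPCCharHealth as a debug message.
; ActorBeginOverlap applies the BPCCharDamage value to any overlapping actor, with no filter for the player.
; CreateHUDEB adds a WBP_EnemyHB widget to the viewport, but nothing in this file calls it.
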(event `self.ReceiveBeginPlay`)

(event `self.ReceiveAnyDamage`
  (params (Damage :type "Float (single-precision)") (DamageType :type "DamageType Object Reference") (InstigatedBy :type "Controller Object Reference") (DamageCauser :type "Actor Object Reference"))
  ;[1 1 1 1 50] ATTACK & DAMAGE - Enemy Base
  ;;[1 1 1] RECEIVE DAMAGE: Toma la función de recibir daño de la clase padre.
  (`parent.ReceiveAnyDamage` Damage DamageType InstigatedBy DamageCauser)
  (`KismetSystemLibrary.PrintString` (`KismetStringLibrary.Concat_StrStr` (`KismetSystemLibrary.GetDisplayName` self) " Health is:" (`KismetStringLibrary.Conv_DoubleToString` (`/Game/Components/BPC_CharHealth.CurrentHealth` (`self.BPC_CharHealth`)))) true true (struct :`G` 0.66 :`B` 1.0 :`A` 1.0) 5.0))

(event `self.ReceiveActorBeginOverlap`
  (params (OtherActor :type "Actor Object Reference"))
  ;[1 1 1 1 50] ATTACK & DAMAGE - Enemy Base
  ;;[1 1 1] COLLISION DAMAGE - Daño por contacto al PJ
  (`GameplayStatics.ApplyDamage` OtherActor (`/Game/Components/BPC_CharDamage.Damage` (`self.BPC_CharDamage`)) null null "/Script/Engine.DamageType"))

(fn `CreateHUDEB`
  (bind _returnvalue (`|CreateWidget` "/Game/Blueprints/Widgets/WBP_EnemyHB.WBP_EnemyHB_C"))
  (`UserWidget.AddToViewport` _returnvalue 3))

(fn `UserConstructionScript`
  (`parent.UserConstructionScript`))