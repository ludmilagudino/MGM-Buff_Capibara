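; BP_Capi is the player character Capi, handling movement, melee and ranged attacks, invulnerable rolls, interaction, damage, death and pause menu.
; Enhanced Input actions play PaperZD override animations, while separate events apply hitbox damage or spawn projectiles.
; A health component feeds the HUD bar.
; Doors teleport Capi behind camera fades and set the pit-fall respawn point, while room entry hands framing to BP_CameraManager.
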(event `self.ReceiveBeginPlay`
  (bind _hitbox (`self.HitBox`))
  ;[1 1 1 1 64] BEGIN PLAY
  (`parent.ReceiveBeginPlay`)
  (bind _asplayer_controller (cast `PlayerController` (`self.GetController`)))
  (`EnhancedInputSubsystemInterface.AddMappingContext` (pcsubsystem `EnhancedInputLocalPlayerSubsystem` _asplayer_controller) "/Game/Entries/InputMapping_Character.InputMapping_Character" 0 (struct))
  ;;[1 1 1 1 36] Crea el HUD del PJ y le añade los valores correspondientes.
  (`self.CreateHUD`)
  (bind (_currenthealth _maxhealth) (`/Game/Components/BPC_CharHealth.initHealth` (`self.BPC_CharHealth`)))
  (`self.UpdateWidget` _currenthealth _maxhealth)
  ;;[1 1 1 1 36] Hace invisible y deshabilita la colisión de la Hit Box de Capi.
  (`SceneComponent.SetHiddenInGame` _hitbox true false)
  (`PrimitiveComponent.SetCollisionEnabled` _hitbox "NoCollision")
  (set `PlayerController.bShowMouseCursor` false (`GameplayStatics.GetPlayerController` 0)))

(event `EnhancedInput|/Game/Entries/Inputs/IA_Pause`
  (params (ActionValue :type Boolean) (ElapsedSeconds :type "Float (double-precision)") (TriggeredSeconds :type "Float (double-precision)") (InputAction :type "InputAction Object Reference" :default "/Game/Entries/Inputs/IA_Pause.IA_Pause"))
  (bind _returnvalue (`GameplayStatics.GetPlayerController` 0))
  ;[1 0.9608 0.7333 1 64] GAME
  ;;[1 1 1 1 50] MENU PAUSA
  (:`Started`
    (if (not (`self.bIsPauseMenuOpen?`))
      (set `self.bIsPauseMenuOpen?` true)
      (bind _returnvalue_2 (`|CreateWidget` "/Game/Blueprints/Widgets/WBP_PauseMenu.WBP_PauseMenu_C" (`GameplayStatics.GetPlayerController` 0)))
      (bind _output_get (set `self.Pause Menu Widget` _returnvalue_2))
      (`UserWidget.AddToViewport` _output_get 0)
      (`WidgetBlueprintLibrary.SetInputMode_GameAndUIEx` _returnvalue (`self.Pause Menu Widget`))
      (set `PlayerController.bShowMouseCursor` true _returnvalue)
      (`GameplayStatics.SetGamePaused` true)
      (else
        (set `self.bIsPauseMenuOpen?` false)
        (`Widget.RemoveFromParent` (`self.Pause Menu Widget`))
        (`GameplayStatics.SetGamePaused` false)
        (`WidgetBlueprintLibrary.SetInputMode_GameOnly` _returnvalue)
        (set `PlayerController.bShowMouseCursor` false _returnvalue)))))

(event `/Game/Blueprints/BPInterfaces/BPI_Door.Door Overlaping`
  (params (DoorLocation :type "Vector Structure") (DoorBoxLocation :type "Vector Structure"))
  ;[0.2794 1 0.9502 1 64] INTERACTIONS
  ;;[1 1 1 1 36] DOORS - USAR PUERTAS - Permite al PJ Capi usar puertas. Las mismas funcionan como teletransportadores. Regula las transciciones.
  (set `self.RoomSpawnPoint` DoorBoxLocation)
  (if (`self.bCanTeleport?`)
    (set `self.bCanTeleport?` false)
    (`self.ChangeCameraZoom` 1200.0)
    (`self.CameraFadeOut`)
    (`self.DisableInput` null)
    (bind _output_get (set `self.PJtoDoorDirection` (`KismetMathLibrary.Normal` (- DoorLocation (`self.K2_GetActorLocation`)))))
    (`self.LaunchCharacter` (* _output_get 300.0))
    (`KismetSystemLibrary.Delay` 1.0)
    (`self.K2_SetActorLocation` DoorBoxLocation false true)
    (`self.CameraFadeIn`)
    (`self.EnableInput` null)
    (`KismetSystemLibrary.Delay` 1.0)
    (set `self.bCanTeleport?` true)))

(event `EnhancedInput|/Game/Entries/Inputs/IA_Move`
  (params (ActionValue :type "Vector2D Structure") (ElapsedSeconds :type "Float (double-precision)") (TriggeredSeconds :type "Float (double-precision)") (InputAction :type "InputAction Object Reference" :default "/Game/Entries/Inputs/IA_Move.IA_Move"))
  (bind (_x _y) (`KismetMathLibrary.BreakVector2D` ActionValue))
  ;[1 1 1 1 64] ACTIONS
  ;;[0.4305 1 0.5236 1 64] MOVEMENT
  ;;;[1 1 1 1 36] WALK: Determina la velocida y dirección del movimiento del personaje. Además guarda la dirección para usar en animaciones.
  (:`Triggered`
    (if (not (`self.bIsRolling?`))
      (set `self.Direction` ActionValue)
      (if (not (`self.bIsAttacking?`))
        (`self.AddMovementInput` (1.0 0.0 0.0) _x)
        (`self.AddMovementInput` (0.0 1.0 0.0) _y)))))

(event `self.ReceiveAnyDamage`
  (params (Damage :type "Float (single-precision)") (DamageType :type "DamageType Object Reference") (InstigatedBy :type "Controller Object Reference") (DamageCauser :type "Actor Object Reference"))
  (bind _bpc_charhealth (`self.BPC_CharHealth`))
  ;[1 1 1 1 64] ACTIONS
  ;;[1 0.6353 0.6452 1 50] ATTACK & DAMAGE - Capi
  ;;;[1 1 1 1 36] RECEIVE DAMAGE: Toma la función de recibir daño de la clase padre. Posteriormente actualiza la vida en el HUD del personaje. Ejecuta la animación de recibir daño. Ejecuta la animación de muerte si la vida llega a 0.
  (`parent.ReceiveAnyDamage` Damage DamageType InstigatedBy DamageCauser)
  (if (not (`self.bIsInvulnerable?`))
    (`self.UpdateWidget` (`/Game/Components/BPC_CharHealth.CurrentHealth` _bpc_charhealth) (`/Game/Components/BPC_CharHealth.MaxHealth` _bpc_charhealth))
    (`PaperZDPlaySlotOverrideAction.PlayAnimationOverrideWithCallbacks` (`PaperZDAnimationComponent.AnimInstance` (`self.AnimationComponent`)) "/Game/Assets/2D/Characters/PJ_Capi/Animations/AnimSequences/Ani_RecieveDamage_CapiPh.Ani_RecieveDamage_CapiPh"
      (:`then`
        _)
      (:`OnCompleted`
        _))
    (if (<= (`/Game/Components/BPC_CharHealth.CurrentHealth` (`self.BPC_CharHealth`)) 0.0)
      (`PaperZDPlaySlotOverrideAction.PlayAnimationOverrideWithCallbacks` (`PaperZDAnimationComponent.AnimInstance` (`self.AnimationComponent`)) "/Game/Assets/2D/Characters/PJ_Capi/Animations/AnimSequences/Ani_Death_CapiPh.Ani_Death_CapiPh"
        (:`OnCompleted`
          _)
        (:`OnCancelled`
          _))
      (`KismetSystemLibrary.DelayUntilNextTick`)
      (`self.K2_DestroyActor`)
      (message `/Game/Blueprints/BPInterfaces/BPI_Player.CapiDead!` (`self.Camera Manager`) false))))

(event `EnhancedInput|/Game/Entries/Inputs/IA_AttackM`
  (params (ActionValue :type Boolean) (ElapsedSeconds :type "Float (double-precision)") (TriggeredSeconds :type "Float (double-precision)") (InputAction :type "InputAction Object Reference" :default "/Game/Entries/Inputs/IA_AttackM.IA_AttackM"))
  (bind _hitbox (`self.HitBox`))
  ;[1 1 1 1 64] ACTIONS
  ;;[1 0.6353 0.6452 1 50] ATTACK & DAMAGE - Capi
  ;;;[1 1 1 1 36] MELEE ATTACK - Ataque básico cuerpo a cuerpo del PJ Capi.
  (:`Triggered`
    (if (`self.bCanAttack?`)
      (if (not (`self.bIsAttacking?`))
        (`PaperZDPlaySlotOverrideAction.PlayAnimationOverrideWithCallbacks` (`PaperZDAnimationComponent.AnimInstance` (`self.AnimationComponent`)) "/Game/Assets/2D/Characters/PJ_Capi/Animations/AnimSequences/Ani_Melee_CapiPh.Ani_Melee_CapiPh" "DefaultSlot" 1.5
          (:`then`
            (set `self.bIsAttacking?` true)
            (`PrimitiveComponent.SetCollisionEnabled` _hitbox "QueryAndPhysics"))
          (:`OnCompleted`
            (set `self.bIsAttacking?` false :!label _label)
            (`SceneComponent.SetHiddenInGame` _hitbox true false)
            (`PrimitiveComponent.SetCollisionEnabled` _hitbox "NoCollision"))
          (:`OnCancelled`
            (goto _label)))))))

(event `EnhancedInput|/Game/Entries/Inputs/IA_Roll`
  (params (ActionValue :type Boolean) (ElapsedSeconds :type "Float (double-precision)") (TriggeredSeconds :type "Float (double-precision)") (InputAction :type "InputAction Object Reference" :default "/Game/Entries/Inputs/IA_Roll.IA_Roll"))
  ;[1 1 1 1 64] ACTIONS
  ;;[0.4305 1 0.5236 1 64] MOVEMENT
  ;;;[1 1 1 1 36] ROLL(DASH) - Permite al PJ Capi realizar un roll. El mismo le permite desplazarse más rápido y esquivar, al desactivar momentaneamente ciertas colisiones.
  (:`Started`
    (set `self.bCanAttack?` false)
    (if (not (`self.bIsRolling?`))
      (set `self.bIsRolling?` true)
      (set `self.bIsInvulnerable?` true)
      (`self.LaunchCharacter` (* (`self.Direction`) (`self.RollSpeed`)) true)
      (`PaperZDPlaySlotOverrideAction.PlayAnimationOverrideWithCallbacks` (`PaperZDAnimationComponent.AnimInstance` (`self.AnimationComponent`)) "/Game/Assets/2D/Characters/PJ_Capi/Animations/AnimSequences/Ani_Roll_CapiPH.Ani_Roll_CapiPH" "DefaultSlot" 1.0 0.3
        (:`OnCompleted`
          (`KismetSystemLibrary.K2_SetTimer` null "EndRoll" (`self.RollDuration`))
          (`KismetSystemLibrary.Delay` 0.1)
          (set `self.bCanAttack?` true))))))

(event `EnhancedInput|/Game/Entries/Inputs/IA_Interact`
  (params (ActionValue :type Boolean) (ElapsedSeconds :type "Float (double-precision)") (TriggeredSeconds :type "Float (double-precision)") (InputAction :type "InputAction Object Reference" :default "/Game/Entries/Inputs/IA_Interact.IA_Interact"))
  ;[0.2794 1 0.9502 1 64] INTERACTIONS
  ;;[1 1 1 1 36] INTERACT - Permite interactuar con elementos e items del nivel como llaves y puertas. Usa la tecla "E".
  (:`Triggered`
    (for _array_element (`self.GetOverlappingActors` "/Script/Engine.Actor")
      (if (`KismetSystemLibrary.DoesImplementInterface` _array_element "/Game/Blueprints/BPInterfaces/BPI_Interact.BPI_Interact_C")
        (message `/Game/Blueprints/BPInterfaces/BPI_Interact.Interact!` _array_element self)
        (break)))))

(event `/Game/Blueprints/BPInterfaces/BPI_Player.CheckAttack`
  ;[1 1 1 1 64] ACTIONS
  ;;[1 0.6353 0.6452 1 50] ATTACK & DAMAGE - Capi
  ;;;[1 1 1 1 36] MELEE ATTACK - Ataque básico cuerpo a cuerpo del PJ Capi.
  (`self.AttackMelee`))

(event `/Game/Blueprints/BPInterfaces/BPI_Sector.EnterRoom`
  (params (`bUsePlayerCam?` :type Boolean) (`Camera Zoom` :type "Float (double-precision)") (`Map Center X` :type "Float (double-precision)") (`Map Center Y` :type "Float (double-precision)") (`Map Location` :type "Vector Structure") (`FollowX?` :type Boolean) (`FollowY?` :type Boolean) (VDoorUp_POS :type "Vector Structure") (VDoorDown_POS :type "Vector Structure") (Cam_YUp_Limit :type "Float (double-precision)") (Cam_YDown_Limit :type "Float (double-precision)"))
  ;[1 0.9608 0.7333 1 64] GAME
  ;;[1 1 1 1 50] CAMERA ZOOM - El circuito completo con BP_Sector y BP_CameraManager modifica el ancho de la cámara, agrega una transcición de 1 segundo aprox.
  (if (not `bUsePlayerCam?`)
    (bind _outactors (`GameplayStatics.GetAllActorsOfClass` "/Game/Blueprints/SectorsAndRooms/BP_CameraManager.BP_CameraManager_C"))
    (bind _output_get (set `self.Camera Manager` (`|GetArrayItem` _outactors)))
    (`PlayerController.SetViewTargetWithBlend` (`GameplayStatics.GetPlayerController` 0) _output_get 0.1 "VTBlend_Linear" 0.0 false)
    (message `/Game/Blueprints/BPInterfaces/BPI_Sector.ChangeCamera` _output_get `Camera Zoom` `Map Center X` `Map Center Y` `Map Location` `FollowX?` `FollowY?` VDoorUp_POS VDoorDown_POS Cam_YUp_Limit Cam_YDown_Limit)))

(event `EnhancedInput|/Game/Entries/Inputs/IA_AttackR`
  (params (ActionValue :type Boolean) (ElapsedSeconds :type "Float (double-precision)") (TriggeredSeconds :type "Float (double-precision)") (InputAction :type "InputAction Object Reference" :default "/Game/Entries/Inputs/IA_AttackR.IA_AttackR"))
  ;[1 1 1 1 64] ACTIONS
  ;;[1 0.6353 0.6452 1 50] ATTACK & DAMAGE - Capi
  ;;;[1 1 1 1 36] RANGE ATTACK -Ataque de rango del PJ Capi.
  (:`Triggered`
    (if (`self.bCanAttack?`)
      (if (not (`self.bIsAttacking?`))
        (`PaperZDPlaySlotOverrideAction.PlayAnimationOverrideWithCallbacks` (`PaperZDAnimationComponent.AnimInstance` (`self.AnimationComponent`)) "/Game/Assets/2D/Characters/PJ_Capi/Animations/AnimSequences/Ani_Range_CapiPh.Ani_Range_CapiPh"
          (:`then`
            (set `self.bIsAttacking?` true))
          (:`OnCompleted`
            (set `self.bIsAttacking?` false :!label _label_2))
          (:`OnCancelled`
            (goto _label_2)))))))

(event `/Game/Blueprints/BPInterfaces/BPI_Capi_Range.Capi Range Attack`
  ;[1 1 1 1 64] ACTIONS
  ;;[1 0.6353 0.6452 1 50] ATTACK & DAMAGE - Capi
  ;;;[1 1 1 1 36] RANGE ATTACK -Ataque de rango del PJ Capi.
  (`self.AttackRange`))

(event `/Game/Blueprints/BPInterfaces/BPI_Hole.Fall`
  (bind _capsulecomponent (`self.CapsuleComponent`))
  ;[1 0.9608 0.7333 1 64] GAME
  ;;[1 1 1 1 36] FALL - Gestiona la secuencia de caida cuando Capi colisiona con un pozo (BP_Hole).
  (if (not (`self.bIsInvulnerable?`))
    (`self.DisableInput` null)
    (`PaperZDPlaySlotOverrideAction.PlayAnimationOverrideWithCallbacks` (`PaperZDAnimationComponent.AnimInstance` (`self.AnimationComponent`)) "/Game/Assets/2D/Characters/PJ_Capi/Animations/AnimSequences/Ani_Fall_CapiPh.Ani_Fall_CapiPh"
      (:`then`
        (`PrimitiveComponent.SetCollisionEnabled` _capsulecomponent "NoCollision")
        (`KismetSystemLibrary.Delay` 1.0)
        (`PrimitiveComponent.SetCollisionEnabled` _capsulecomponent "QueryAndPhysics")
        (`self.K2_SetActorLocation` (`self.RoomSpawnPoint`))
        (`self.EnableInput` null)
        (`GameplayStatics.ApplyDamage` self 10.0)))))

(event `EnhancedInput|/Game/Entries/Inputs/IA_Run`
  (params (ActionValue :type Boolean) (ElapsedSeconds :type "Float (double-precision)") (TriggeredSeconds :type "Float (double-precision)") (InputAction :type "InputAction Object Reference" :default "/Game/Entries/Inputs/IA_Run.IA_Run"))
  ;[1 0.6696 0.3033 1 36] OLD
  ;;[0.5748 0.7806 1] SPRINT: Duplica la velocidad máxima al apretar Shift izquierdo y la reduce a la mitad al soltar.
)

(event `self.HitBox.OnComponentBeginOverlap`
  (params (OverlappedComponent :type "PrimitiveComponent Object Reference") (OtherActor :type "Actor Object Reference") (OtherComp :type "PrimitiveComponent Object Reference") (OtherBodyIndex :type Integer) (bFromSweep :type Boolean) (SweepResult :type "HitResult Structure (by ref)"))
  ;[1 0.6696 0.3033 1 36] OLD
  ;;[1 1 1 1 36] MELEE ATTACK
)

(event `EnhancedInput|/Game/Entries/Inputs/IA_AttackM`
  (params (ActionValue :type Boolean) (ElapsedSeconds :type "Float (double-precision)") (TriggeredSeconds :type "Float (double-precision)") (InputAction :type "InputAction Object Reference" :default "/Game/Entries/Inputs/IA_AttackM.IA_AttackM"))
  ;[1 0.6696 0.3033 1 36] OLD
  ;;[1 1 1 1 36] MELEE ATTACK
)

(event `EnhancedInput|/Game/Entries/Inputs/IA_Jump`
  (params (ActionValue :type Boolean) (ElapsedSeconds :type "Float (double-precision)") (TriggeredSeconds :type "Float (double-precision)") (InputAction :type "InputAction Object Reference" :default "/Game/Entries/Inputs/IA_Jump.IA_Jump"))
  ;[1 0.6696 0.3033 1 36] OLD
  ;;[1 0.9451 0.349] JUMP: Desplazamineto vertical.
)

(fn `AttackMelee`
  (for _array_element (`PrimitiveComponent.GetOverlappingActors` (`self.HitBox`) "/Game/Blueprints/Enemies/BP_EnemyBaseZD.BP_EnemyBaseZD_C")
    (`GameplayStatics.ApplyDamage` _array_element (`/Game/Components/BPC_CharDamage.Damage` (`self.BPC_CharDamage`)))
    (`GameplayStatics.PlaySound2D` "/Game/Assets/Sound/FX/CapiAtaquesYDMG/MeleWoosh_And_Impact/MS_Hit.MS_Hit" 0.5 1.0 0.0 null null)))

(fn `AttackRange`
  (bind (_returnvalue_x _returnvalue_y) (`KismetMathLibrary.BreakVector` (+ (`self.K2_GetActorLocation`) (* (`self.GetActorForwardVector`) 100.0))))
  (`|SpawnActorFromClass` "/Game/Blueprints/Playable_Characters/BP_Projectile_Capi.BP_Projectile_Capi_C" (`KismetMathLibrary.MakeTransform` (`KismetMathLibrary.MakeVector` _returnvalue_x _returnvalue_y 50.0) (`KismetMathLibrary.MakeRotFromX` (`self.GetActorForwardVector`))) "Undefined" "MultiplyWithRoot" null (10.0 0.0 0.0) self))

(fn `CameraFadeIn`
  (`PlayerCameraManager.StartCameraFade` (`PlayerController.PlayerCameraManager` (`GameplayStatics.GetPlayerController` 0)) 1.0 0.0 0.5 (struct :`R` 0.088542 :`G` 0.037076 :`B` 0.008216 :`A` 1.0) false true))

(fn `CameraFadeOut`
  (`PlayerCameraManager.StartCameraFade` (`PlayerController.PlayerCameraManager` (`GameplayStatics.GetPlayerController` 0)) 0.0 1.0 1.0 (struct :`R` 0.088542 :`G` 0.037076 :`B` 0.008216 :`A` 1.0) false true))

(fn `ChangeCameraZoom`
  (params (NewCameraWidth :type "Float (double-precision)" :default 1200.0))
  (set `self.Camera_Width` (`CameraComponent.OrthoWidth` (`self.Camera1`)))
  (bind _output_get (set `self.New_Camera_Width` NewCameraWidth))
  (set `self.Camera_Width` _output_get))

(fn `CreateHUD`
  (locals (NewLocalVar :type "/Game/Blueprints/Widgets/WBP_HUD Object Reference"))
  (bind _bpc_charhealth (`self.BPC_CharHealth`))
  (bind _returnvalue (`|CreateWidget` "/Game/Blueprints/Widgets/WBP_HUD.WBP_HUD_C" (`GameplayStatics.GetPlayerController` 0)))
  (`UserWidget.AddToViewport` _returnvalue 0)
  (bind _output_get (set `self.WBP_HUD` _returnvalue))
  (bind _wpb_healthbar (`/Game/Blueprints/Widgets/WBP_HUD.WPB_HealthBar` _output_get))
  (`ProgressBar.SetPercent` (`/Game/Blueprints/Widgets/WPB_HealthBar.ProgressBar_Health` _wpb_healthbar) (/ (`/Game/Components/BPC_CharHealth.CurrentHealth` _bpc_charhealth) (`/Game/Components/BPC_CharHealth.MaxHealth` _bpc_charhealth)))
  (set `TextBlock.Text` (`KismetTextLibrary.Conv_DoubleToText` 0.0 "HalfToEven") (`/Game/Blueprints/Widgets/WPB_HealthBar.TextCurrentHealth` _wpb_healthbar))
  (set `TextBlock.Text` (`KismetTextLibrary.Conv_DoubleToText` 0.0 "HalfToEven") (`/Game/Blueprints/Widgets/WPB_HealthBar.TextMaxHealth` _wpb_healthbar)))

(fn `Cure`
  (params (Cure :type "Float (double-precision)"))
  (bind _bpc_charhealth (`self.BPC_CharHealth`))
  (bind _maxhealth (`/Game/Components/BPC_CharHealth.MaxHealth` _bpc_charhealth))
  (bind _returnvalue (`KismetMathLibrary.FClamp` (+ Cure (`/Game/Components/BPC_CharHealth.CurrentHealth` _bpc_charhealth)) 0.0 _maxhealth))
  (set `/Game/Components/BPC_CharHealth.CurrentHealth` _returnvalue _bpc_charhealth)
  (`self.UpdateWidget` _returnvalue _maxhealth))

(fn `EndRoll`
  (set `self.bIsRolling?` false)
  (set `self.bIsInvulnerable?` false)
  (`MovementComponent.StopMovementImmediately` (`self.CharacterMovement`)))

(fn `Teleported!`
  (returns (CanTeleport :type Boolean))
  (return false))

(fn `UpdateWidget`
  (params (CurrentHealth :type "Float (double-precision)") (MaxHealth :type "Float (double-precision)"))
  (`/Game/Blueprints/Widgets/WPB_HealthBar.UpdateW` (`/Game/Blueprints/Widgets/WBP_HUD.WPB_HealthBar` (`self.WBP_HUD`)) CurrentHealth MaxHealth))

(fn `UserConstructionScript`
  (`parent.UserConstructionScript`))